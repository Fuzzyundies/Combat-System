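; Player state Blueprint that tracks a sword guard position and an intent for directional melee.
; SwitchPosition thresholds mouse X/Y into a two-letter string mapped to eight outer positions, with center keeping the current one.
; SwitchIntent picks between two intents by mouse wheel direction.
; Changes print to screen and set lock flags, which Tick-driven listeners release after a short delay to throttle switching.
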(event `self.ReceiveBeginPlay`)

(event `self.ReceiveTick`
  (params (DeltaSeconds :type "Float (single-precision)"))
  (`|ExecutionSequence`
    (:`then_0`
      (`self.PositionLockListener`))
    (:`then_1`
      (`self.IntentLockListener`))))

(fn `CheckCLR`
  (params (Left :type Boolean) (Right :type Boolean))
  (bind _stancestring (`self.StanceString`))
  (if Left
    (set `self.StanceString` (`KismetStringLibrary.Concat_StrStr` _stancestring "L"))
    (elif Right
      (set `self.StanceString` (`KismetStringLibrary.Concat_StrStr` _stancestring "R"))
      (else
        (set `self.StanceString` (`KismetStringLibrary.Concat_StrStr` _stancestring "C")))))
  (return))

(fn `CheckTMB`
  (params (Top :type Boolean) (Bottom :type Boolean))
  (if Top
    (set `self.StanceString` "T")
    (elif Bottom
      (set `self.StanceString` "B")
      (else
        (set `self.StanceString` "M"))))
  (return))

(fn `ClearPositionAndIntent`
  (set `self.SwordPosition` "NewEnumerator0")
  (set `self.Intent` "NewEnumerator2"))

(fn `SwitchIntent`
  (params (MouseWheel :type "Float (double-precision)"))
  (if (not (`self.Change Intent`))
    (if (> MouseWheel 0.0)
      (set `self.PreviousIntent` (`self.Intent`))
      (set `self.Intent` "NewEnumerator0")
      ;[1 1 1] Attempt at small measures of efficiency in terms of the if statement.
      (if (not (`|EnumEquality` (`self.Intent`) (`self.PreviousIntent`))) :!label _label
        (set `self.Change Intent` true)
        (`self.UpdateGuardAndIntent`))
      (elif (< MouseWheel 0.0)
        (set `self.PreviousIntent` (`self.Intent`))
        (set `self.Intent` "NewEnumerator1")
        (goto _label)))))

(fn `SwitchPosition`
  (params (`Mouse X` :type "Float (double-precision)") (`Mouse Y` :type "Float (double-precision)") (`Moust Tolerance` :type "Float (double-precision)"))
  (bind _returnvalue (* `Moust Tolerance` -1.0))
  (if (not (`self.Change Position`))
    (`self.CheckTMB` (<= `Mouse Y` _returnvalue) (>= `Mouse Y` `Moust Tolerance`))
    (`self.CheckCLR` (<= `Mouse X` _returnvalue) (>= `Mouse X` `Moust Tolerance`))
    (set `self.PreviousPosition` (`self.SwordPosition`))
    (switch `string` (`self.StanceString`)
      (:`TL`
        (set `self.SwordPosition` "NewEnumerator1"))
      (:`TC`
        (set `self.SwordPosition` "NewEnumerator2"))
      (:`TR`
        (set `self.SwordPosition` "NewEnumerator3"))
      (:`ML`
        (set `self.SwordPosition` "NewEnumerator4"))
      (:`MC`
        _)
      (:`MR`
        (set `self.SwordPosition` "NewEnumerator6"))
      (:`BL`
        (set `self.SwordPosition` "NewEnumerator7"))
      (:`BC`
        (set `self.SwordPosition` "NewEnumerator5"))
      (:`BR`
        (set `self.SwordPosition` "NewEnumerator8")))
    (if (not (`|EnumEquality` (`self.SwordPosition`) (`self.PreviousPosition`)))
      (set `self.Change Position` true)
      (`self.UpdateGuardAndIntent`))))

(fn `UpdateGuardAndIntent`
  (`KismetSystemLibrary.PrintString` (`KismetStringLibrary.Concat_StrStr` "Position:" (`|GetEnumeratorNameAsString` (`self.SwordPosition`)) " " "Intent:" (`|GetEnumeratorNameAsString` (`self.Intent`)))))

(fn `UserConstructionScript`)